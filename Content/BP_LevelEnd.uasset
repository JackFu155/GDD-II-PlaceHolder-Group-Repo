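; BP_LevelEnd is a level-end trigger that finishes the level when the side-scroller player character overlaps it.
; On overlap it casts to the character and MagnetManGameInstance, copies the collectable count and total play time into the game instance's score variables, then opens the GameOver level.
; Leftover unconnected nodes for setting a collectable maximum and debug-printing the score never run.
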(event `self.ReceiveActorBeginOverlap`
  (params (OtherActor :type "Actor Object Reference"))
  (bind _as2dside_scroller_character (cast `/Game/2DSideScrollerBP/Blueprints/2DSideScrollerCharacter` OtherActor))
  (bind _asmagnet_man_game_instance (cast `/Game/MagnetManGameInstance` (`GameplayStatics.GetGameInstance`)))
  (`|ExecutionSequence`
    (:`then_0`
      (set `/Game/MagnetManGameInstance.CollectableScore` (`/Game/2DSideScrollerBP/Blueprints/2DSideScrollerCharacter.CollectableCount` _as2dside_scroller_character) _asmagnet_man_game_instance))
    (:`then_2`
      (set `/Game/MagnetManGameInstance.TimeScore` (`/Game/2DSideScrollerBP/Blueprints/2DSideScrollerCharacter.totalPlayTime` _as2dside_scroller_character) _asmagnet_man_game_instance))
    (:`then_3`
      (`GameplayStatics.OpenLevel` "GameOver"))))

(fn `UserConstructionScript`)